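; Prisoner character Blueprint that lets the player open and close cell doors and grab or release objects.
; While the Grabber allows hacking, Tick sphere-scans nearby dynamic objects and keeps the last as Target.
; Keyboard or gamepad input toggles a CellDoor-tagged Target via timeline lerps, or toggles the Grabber.
; BeginPlay stores one shared start and X-offset open location, overwritten per door, so the last door found sets both.
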(event `Key|Gamepad_FaceButton_Top`
  (params (Key :type "Key Structure"))
  (bind _target (`self.Target`))
  (:`Pressed`
    (if (`self.ActorHasTag` (`self.Target`) "CellDoor") :!label _label
      (if (`self.IsOpen`)
        (bind (_direction _newtrack_0) (`Timeline|Timeline`)
          (:`Update`
            (`self.K2_SetActorLocation` _target (`KismetMathLibrary.VLerp` (`self.K2_GetActorLocation` _target) (`self.StartLocation`) _newtrack_0) false false)
            (set `self.IsOpen` false)))
        (else
          (bind (_direction_2 _newtrack_0_2) (`Timeline|Timeline_OpenDoor`)
            (:`Update`
              (`self.K2_SetActorLocation` _target (`KismetMathLibrary.VLerp` (`self.StartLocation`) (`self.TargetLocation`) _newtrack_0_2) false false)
              (set `self.IsOpen` true))))))))

(event `self.ReceiveBeginPlay`
  (bind _outactors (`GameplayStatics.GetAllActorsWithTag` "CellDoor"))
  (for _array_element _outactors
    (bind _output_get (set `self.StartLocation` (`self.K2_GetActorLocation` _array_element)))
    (set `self.TargetLocation` (`KismetMathLibrary.MakeVector` (+ (`self.MoveDoor`) (.x _output_get)) (.y _output_get) (.z _output_get)))))

(event `Key|C`
  (params (Key :type "Key Structure"))
  (:`Pressed`
    (goto _label)))

(event `self.ReceiveActorBeginOverlap`
  (params (OtherActor :type "Actor Object Reference")))

(event `self.ReceiveTick`
  (params (DeltaSeconds :type "Float (single-precision)"))
  (if (`Grabber.CanHackDoor` (`self.Grabber`))
    (bind _outactors (`KismetSystemLibrary.SphereOverlapActors` (`self.K2_GetActorLocation`) 150.0 (`|MakeArray` "ObjectTypeQuery2" :!type "EObjectTypeQuery Enum")))
    (for _array_element _outactors
      (set `self.Target` _array_element))))

(event `Key|G`
  (params (Key :type "Key Structure"))
  (bind _grabber (`self.Grabber`))
  ;[1 1 1] Grab function
  (:`Pressed`
    (if (`self.IsGrabbing`) :!label _label_2
      (`Grabber.ReleaseObject` _grabber)
      (set `self.IsGrabbing` false)
      (else
        (`Grabber.GrabObject` _grabber)
        (set `self.IsGrabbing` true)))))

(event `Key|Gamepad_FaceButton_Left`
  (params (Key :type "Key Structure"))
  ;[1 1 1] Grab function
  (:`Pressed`
    (goto _label_2)))

(fn `DetectHackableObjects`
  (bind _outactors (`KismetSystemLibrary.SphereOverlapActors` (`self.K2_GetActorLocation`) 150.0 (`|MakeArray` "ObjectTypeQuery2" :!type "EObjectTypeQuery Enum")))
  (for _array_element _outactors
    (bind _output_get (set `self.Target` _array_element))))

(fn `UserConstructionScript`)